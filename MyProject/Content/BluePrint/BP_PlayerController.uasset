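; BP_PlayerController is a player controller that translates axis input into movement and look control for the player's BP_MyCharactor pawn.
; On BeginPlay it casts player pawn 0 to BP_MyCharactor and caches the reference.
; Axis events feed movement input along the character's forward and right vectors, plus controller yaw and pitch for looking.
; Only the forward/backward handler validity-checks the cached reference before using it.
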(event EventBeginPlay
  ;[1 1 1] Controller
  (bind _asbp_my_charactor (Utilities|Casting|CastToBP_MyCharactor (Game|Player|GetPlayerPawn 0)))
  (Variables|Default|SetAs%20BP%20My%20Charactor _asbp_my_charactor))

(event EventTick
  (params (DeltaSeconds :type Float%20%28single-precision%29)))

(event Input|AxisEvents|InputAxisMoveForwardBackward
  (params (AxisValue :type Float%20%28single-precision%29))
  (bind _as_bp_my_charactor (Variables|Default|GetAs%20BP%20My%20Charactor))
  ;[1 1 1] Move Forward & Backward
  (Utilities|IsValid _as_bp_my_charactor
    (:Is%20Valid
      (Pawn|Input|AddMovementInput (Variables|Default|GetAs%20BP%20My%20Charactor) (Transformation|GetActorForwardVector _as_bp_my_charactor) AxisValue false))))

(event Input|AxisEvents|InputAxisMoveLeftRight
  (params (AxisValue :type Float%20%28single-precision%29))
  ;[1 1 1] Move Left & Right
  (Pawn|Input|AddMovementInput (Variables|Default|GetAs%20BP%20My%20Charactor) (Transformation|GetActorRightVector (Variables|Default|GetAs%20BP%20My%20Charactor)) AxisValue false))

(event Input|AxisEvents|InputAxisRotate
  (params (AxisValue :type Float%20%28single-precision%29))
  ;[1 1 1] Rotate
  (Pawn|Input|AddControllerYawInput (Variables|Default|GetAs%20BP%20My%20Charactor) AxisValue))

(event Input|AxisEvents|InputAxisLookUP
  (params (AxisValue :type Float%20%28single-precision%29))
  ;[1 1 1] Rotate
  (Pawn|Input|AddControllerPitchInput (Variables|Default|GetAs%20BP%20My%20Charactor) AxisValue))

(fn ConstructionScript)